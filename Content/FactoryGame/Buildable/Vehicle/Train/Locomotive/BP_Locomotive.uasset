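; BP_Locomotive is the player-drivable train locomotive, laid out here as a stub with empty event bodies and construction script.
; It declares hooks for driving input, possession, camera updates, train naming and significance changes.
; Two horns have start and stop events in paired Server and MultiCast forms, with no wiring between them.
; Map and compass representation functions return placeholder values such as false, empty text and zero vectors.
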(event Custom|InpActEvt_Use_K2Node_InputActionEvent_3
  (params (Key :type Key%20Structure :default "None")))

(event Custom|InpActEvt_Jump_Drift_K2Node_InputActionEvent_2
  (params (Key :type Key%20Structure :default "None")))

(event Custom|MultiCast_TrainHorn_01)

(event Custom|MultiCast_TrainHorn_01_Stop)

(event Custom|MultiCast_TrainHorn_02)

(event Custom|MultiCast_TrainHorn_02_Stop)

(event Custom|Server_Horn_01)

(event Custom|Server_Horn_01_Stop)

(event Custom|Server_Horn_02)

(event Custom|Server_Horn_02_Stop)

(event Custom|UpdateTrainName)

(event Custom|InpActEvt_Jump_Drift_K2Node_InputActionEvent_1
  (params (Key :type Key%20Structure :default "None")))

(event Custom|InpActEvt_ResourceScanner_ToggleVehicleRecording_K2Node_InputActionEvent_0
  (params (Key :type Key%20Structure :default "None")))

(event Custom|InpActEvt_LeftMouseButton_K2Node_InputKeyEvent_1
  (params (Key :type Key%20Structure :default "None")))

(event Custom|InpActEvt_LeftMouseButton_K2Node_InputKeyEvent_0
  (params (Key :type Key%20Structure :default "None")))

(event Custom|UpdateCamera)

(event Custom|Server_Leave)

(event Custom|InpAxisEvt_MoveRight_K2Node_InputAxisEvent_0
  (params (AxisValue :type Float%20%28single-precision%29)))

(event Custom|InpAxisEvt_MoveForward_K2Node_InputAxisEvent_1
  (params (AxisValue :type Float%20%28single-precision%29)))

(event EventBeginPlay)

(event Collision|EventActorBeginOverlap
  (params (OtherActor :type Actor%20Object%20Reference)))

(event EventTick
  (params (DeltaSeconds :type Float%20%28single-precision%29)))

(event EventDestroyed)

(event EventUnpossessed
  (params (OldController :type Controller%20Object%20Reference)))

(event EventPossessed
  (params (NewController :type Controller%20Object%20Reference)))

(event EventOnNameChanged)

(event EventGainedSignificance)

(event EventLostSignificance)

(fn ConstructionScript)

(fn AddasRepresentation
  (return false))

(fn GetActorCompassViewDistance
  (return "CVD_Off"))

(fn GetActorFogOfWarRevealRadius
  (return 0.0))

(fn GetActorFogOfWarRevealType
  (return "FOWRT_None"))

(fn GetActorRepresentationColor
  (return ""))

(fn GetActorRepresentationText
  (return ""))

(fn GetActorRepresentationTexture
  (return 0))

(fn GetActorRepresentationType
  (return "RT_Default"))

(fn GetActorShouldShowinCompass
  (return false))

(fn GetActorShouldShowonMap
  (return false))

(fn GetRealActorLocation
  (return "0, 0, 0"))

(fn GetRealActorRotation
  (return "0, 0, 0"))

(fn IsActorStatic
  (return false))

(fn RemoveasRepresentation
  (return false))

(fn SetActorCompassViewDistance
  (params (compassViewDistance :type ECompassViewDistance%20Enum :default "CVD_Off"))
  (return "CVD_Off"))

(fn SetActorRepresentationText
  (params (newText :type Text%20%28by%20ref%29))
  (return ""))

(fn UpdateRepresentation
  (return false))